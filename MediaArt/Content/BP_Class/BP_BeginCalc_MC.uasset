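; Actor Blueprint that shows an on-screen elapsed-time counter through a UI_Timer_MC widget created at BeginPlay.
; While IsPrint is false, Tick accumulates delta seconds in CurTime and writes "min : sec" text to the widget.
; Minutes are the unfloored CurTime / 60, and seconds are the remainder rounded to two digits.
; A "Game Over" check that would set IsPrint and a debug arithmetic print are disconnected and never run.
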(event EventBeginPlay
  (bind _returnvalue (UserInterface|CreateWidget "/Game/BP_Class/UI_Timer_MC.UI_Timer_MC_C" (Game|GetPlayerController 0)))
  (bind _output_get (Variables|Default|SetuiTimerObj _returnvalue))
  (UserInterface|Viewport|AddtoViewport _output_get 0)
  (Variables|/Game/BP_Class/UI_Timer_MC.UI_Timer_MC_C|SetuiTimeText _output_get "Test"))

(event Collision|EventActorBeginOverlap
  (params (OtherActor :type Actor%20Object%20Reference)))

(event EventTick
  (params (DeltaSeconds :type Float%20%28single-precision%29))
  ;[0.15 0.15 0.15 0.5] Timer를 만들자!
  (if (not (Variables|Default|GetisPrint))
    (bind _output_get (Variables|Default|SetcurTime (+ DeltaSeconds (Variables|Default|GetcurTime)))) ; set
    (Variables|/Game/BP_Class/UI_Timer_MC.UI_Timer_MC_C|SetuiTimeText (Variables|Default|GetuiTimerObj) (Utilities|Text|FormatText "{min} : {sec}" (Utilities|Text|ToText(Float) (/ _output_get 6e+01) "ToZero" false true 2 2 0 0) (Utilities|Text|ToText(Float) (Math|Float|%(Float) _output_get 6e+01) "HalfToEven" false true 2 2 0 0)))))

(fn ConstructionScript)